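; Game mode for an endless runner in which the player is followed by an AI-possessed chaser.
; A setup state switch runs from pre-game to in-game, spawning controller, map, runner and chaser, then starting looping speed-increase timers and audio.
; The track chains random platforms via each tile's spawn point, with a helper to destroy the oldest.
; It binds the runner's killed event and can show a results screen; score setup and post-game are empty.
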(event Custom|PreGame
  (CallFunction|SetupCharacter)
  (CallFunction|SpawnAIController)
  (CallFunction|SwitchGameSetUp "NewEnumerator1"))

(event Custom|SetUp
  (CallFunction|SetUpRunnerMap)
  (CallFunction|SpawnCharacter)
  (CallFunction|SetUpScore)
  (CallFunction|SpawnChaser)
  (CallFunction|SwitchGameSetUp "NewEnumerator2"))

(event Custom|InGame
  (CallFunction|IncreasePlayerSpeedAfterDuration)
  (Audio|PlaySound2D "/Game/Jamie/Skydiving__Loopable__Cue.Skydiving__Loopable__Cue" 1.0 1.0 0.0 0 0))

(event Custom|PostGame)

(event EventBeginPlay
  (CallFunction|SwitchGameSetUp "NewEnumerator0"))

(fn ConstructionScript)

(fn SwitchGameSetUp
  (params (Set%20Up%20Mode :type Enum_GameStartUp%20Enum :default "NewEnumerator0"))
  (switch Utilities|FlowControl|Switch|SwitchonEnum_GameStartUp Set%20Up%20Mode
    (:NewEnumerator0
      (CallFunction|PreGame))
    (:NewEnumerator1
      (CallFunction|SetUp))
    (:NewEnumerator2
      (CallFunction|InGame))
    (:NewEnumerator3
      (CallFunction|PostGame))))

(fn SpawnTile
  (bind _returnvalue (Game|SpawnActorfromClass (.OutItem (Utilities|Array|Random (Variables|Default|GetPlatforms))) (Variables|Default|GetNextSpawnPoint) "Undefined" 0 0))
  (Utilities|Array|Add (Variables|Default|GetActivePlatforms) _returnvalue)
  (Variables|Default|SetNextSpawnPoint (Transformation|GetWorldTransform (Variables|/Game/Jamie/Blueprint/Platforms/BP_BasePlatform.BP_BasePlatform_C|GetSpawnPoint _returnvalue))))

(fn SetUpRunnerMap
  (bind _returnvalue (Game|SpawnActorfromClass (Variables|Default|GetSetUpPlatform) (Variables|Default|GetNextSpawnPoint) "Undefined" 0 0))
  (Utilities|Array|Add (Variables|Default|GetActivePlatforms) _returnvalue)
  (Variables|Default|SetNextSpawnPoint (Transformation|GetWorldTransform (Variables|/Game/Jamie/Blueprint/Platforms/BP_BasePlatform.BP_BasePlatform_C|GetSpawnPoint _returnvalue)))
  (for _index (range 1 (Variables|Default|GetPlatformRenderDistance))
    (CallFunction|SpawnTile)))

(fn RemoveLastPlatform
  (bind _activeplatforms (Variables|Default|GetActivePlatforms))
  (LocalVariables|SetLastPlatform (Utilities|Array|Get(acopy) _activeplatforms))
  (Utilities|Array|RemoveIndex _activeplatforms)
  (Actor|DestroyActor (LocalVariables|GetLastPlatform)))

(fn SpawnCharacter
  (bind _returnvalue (Game|SpawnActorfromClass "/Game/Dan/Player/BP_RunnerCharacter.BP_RunnerCharacter_C" (Math|Transform|MakeTransform (+ (.location (Transformation|GetWorldTransform (Variables|/Game/Jamie/Blueprint/Platforms/BP_StartingPlatform.BP_StartingPlatform_C|GetStartingPoint (.AsBP%20Starting%20Platform (Utilities|Casting|CastToBP_StartingPlatform (Utilities|Array|Get(acopy) (Variables|Default|GetActivePlatforms))))))) "0,0,100.000000") "0, 0, 0" "1.000000,1.000000,1.000000") "Undefined" 0 0))
  (bind _output_get (Variables|Default|SetRunnerCharacter _returnvalue))
  (Pawn|Possess (Variables|Default|GetplayerController) _output_get)
  (EventDispatchers|BindEventtoPlayerKilled (Variables|Default|GetRunnerCharacter) (EventDispatchers|CreateEvent :!event CreateResultsScreen)))

(fn SetupCharacter
  (Variables|Default|SetplayerController (Game|GetPlayerController 0)))

(fn SetUpScore)

(fn IncreasePlayerSpeedAfterDuration
  (Utilities|Time|SetTimerbyEvent (EventDispatchers|CreateEvent (Variables|Default|GetRunnerCharacter) :!event IncreaseSpeed) (Variables|Default|GetSpeedIncreaseDelay) true)
  (Utilities|Time|SetTimerbyEvent (EventDispatchers|CreateEvent (Variables|Default|GetChaser) :!event IncreaseSpeed) (Variables|Default|GetSpeedIncreaseDelay) true))

(fn SpawnChaser
  (bind _activeplatforms (Variables|Default|GetActivePlatforms))
  (bind _output (Utilities|Array|Get(acopy) _activeplatforms))
  (bind _asbp_starting_platform (Utilities|Casting|CastToBP_StartingPlatform _output))
  (bind _startingpoint (Variables|/Game/Jamie/Blueprint/Platforms/BP_StartingPlatform.BP_StartingPlatform_C|GetStartingPoint _asbp_starting_platform))
  (bind _returnvalue (Transformation|GetWorldTransform _startingpoint))
  (bind _returnvalue_2 (Game|SpawnActorfromClass "/Game/Dan/AI/BP_Chaser.BP_Chaser_C" (Math|Transform|MakeTransform (Math|Vector|MakeVector (- (.x (.location _returnvalue)) 325.0) (.y (.location _returnvalue)) (+ (.z (.location _returnvalue)) 1e+02)) "0, 0, 0" "1.000000,1.000000,1.000000") "Undefined" 0 0))
  (Variables|Default|SetChaser _returnvalue_2)
  (Pawn|Possess (Variables|Default|GetAIController) _returnvalue_2)
  (Variables|/Game/Dan/Player/BP_RunnerCharacter.BP_RunnerCharacter_C|Setchaser (Variables|Default|GetRunnerCharacter) _returnvalue_2))

(fn SpawnAIController
  (bind _returnvalue (Game|SpawnActorfromClass "/Game/Dan/AI/BP_AI_Contoller.BP_AI_Contoller_C" (Math|Transform|MakeTransform "0, 0, 0" "0, 0, 0" "1.000000,1.000000,1.000000") "Undefined" 0 0))
  (Variables|Default|SetAIController _returnvalue))

(fn CreateResultsScreen
  (params (Score :type Integer) (Credits :type Integer))
  (bind _returnvalue (UserInterface|CreateWidget "/Game/UI/gameover/gameover-playagain.gameover-playagain_C"))
  (bind _output_get (Variables|Default|SetResultsScreen _returnvalue))
  (UserInterface|Viewport|AddtoViewport _output_get 0)
  (Default|InitResults _output_get Score Credits))