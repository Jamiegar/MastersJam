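; Base platform tile for a runner game that places an obstacle on itself and drives the track's recycling.
; On BeginPlay it spawns one BP_Obstacle at a random X within the Cube's bounds and a random YAxisPoints entry.
; Attaching with KeepRelative turns that spawn position into a platform-local offset.
; When the runner overlaps the Box, GM_Runner spawns a new tile and removes the last platform.
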(event OnComponentBeginOverlap(Box)
  (params (OverlappedComponent :type Primitive%20Component%20Object%20Reference) (OtherActor :type Actor%20Object%20Reference) (OtherComp :type Primitive%20Component%20Object%20Reference) (OtherBodyIndex :type Integer) (bFromSweep :type Boolean) (SweepResult :type Hit%20Result%20Structure%20%28by%20ref%29))
  (if (!= OtherActor "BP_BasePlatform")
    (Utilities|Casting|CastToBP_RunnerCharacter OtherActor)
    (bind _asgm_runner (Utilities|Casting|CastToGM_Runner (Game|GetGameMode)))
    (Default|SpawnTile _asgm_runner)
    (Default|RemoveLastPlatform _asgm_runner)))

(event EventBeginPlay
  (bind _localpos (CallFunction|GetRandomXSurfaceLocation))
  (CallFunction|SpawnObstacle _localpos))

(fn ConstructionScript)

(fn GetRandomXSurfaceLocation
  (bind _cube (Variables|Default|GetCube))
  (bind (_min _max) (Components|StaticMesh|GetLocalBounds _cube))
  (return (Math|Vector|MakeVector (Math|Random|RandomFloatinRange (.X (Math|Vector|BreakVector _min)) (.X (Math|Vector|BreakVector _max))) (.OutItem (Utilities|Array|Random (Variables|Default|GetYAxisPoints))) 8e+01)))

(fn SpawnObstacle
  (params (LocalPosOnPlatform :type Vector))
  (bind _returnvalue (Game|SpawnActorfromClass "/Game/Jamie/Blueprint/Obstacles/BP_Obstacle.BP_Obstacle_C" (Math|Transform|MakeTransform LocalPosOnPlatform "0, 0, 0" "1.000000,1.000000,1.000000") "Undefined" 0 0))
  (Transformation|AttachActorToActor _returnvalue self "None" "KeepRelative" "KeepRelative" "KeepRelative" true))