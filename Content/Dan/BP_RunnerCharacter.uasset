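; BP_RunnerCharacter is a lane-based runner character that moves forward automatically while the player switches lanes.
; A and D key presses teleport it sideways along world Y in fixed steps, using exact position checks to block moves past the outer lanes.
; Tick prints the actor location for debugging, then adds forward movement input scaled by MoveSpeed.
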(event EventTick
  (params (DeltaSeconds :type Float%20%28single-precision%29))
  (Utilities|FlowControl|Sequence
    (:then_0
      (Development|PrintString (Utilities|String|ToString(Vector) (Transformation|GetActorLocation)) true true "(R=0.000000,G=0.660000,B=1.000000,A=1.000000)" 0.0))
    (:then_1
      (Pawn|Input|AddMovementInput (Transformation|GetActorForwardVector) (Variables|Default|GetMoveSpeed) false))))

(event Input|KeyboardEvents|A
  (params (Key :type Key%20Structure :default "None"))
  (bind _returnvalue (Transformation|GetActorLocation))
  (:Pressed
    (if (not (== (.y (Transformation|GetActorLocation)) -2e+02))
      (Transformation|SetActorLocation (Math|Vector|MakeVector (.x _returnvalue) (- (.y _returnvalue) 2e+02) (.z _returnvalue)) false false))))

(event Input|KeyboardEvents|D
  (params (Key :type Key%20Structure :default "None"))
  (bind _returnvalue (Transformation|GetActorLocation))
  (:Pressed
    (if (not (== (.y (Transformation|GetActorLocation)) 2e+02))
      (Transformation|SetActorLocation (Math|Vector|MakeVector (.x _returnvalue) (+ (.y _returnvalue) 2e+02) (.z _returnvalue)) false false))))

(fn ConstructionScript)