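; BP_Chaser is an AI character that constantly runs forward and mirrors player moves, apparently as the pursuer in a lane-based runner.
; Player move events drive jumps or timeline lerps that shift it sideways along world Y by a fixed lane step.
; IncreaseSpeed compounds walk speed by a percentage up to MaxSpeed and adds a small forward launch.
; BeginPlay randomly gives its Photo one of two face materials, Greg or Stu.
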(event EventPlayerJumped
  (Character|Jump))

(event EventBeginPlay
  (switch int (Math|Random|RandomIntegerinRange 0 1)
    (:0
      (Rendering|Material|SetMaterial (Variables|Default|Getphoto) 0 "/Game/Dan/AI/greg_Mat.greg_Mat"))
    (:1
      (Rendering|Material|SetMaterial (Variables|Default|Getphoto) 0 "/Game/Dan/AI/stu_Mat.stu_Mat"))))

(event EventTick
  (params (DeltaSeconds :type Float%20%28single-precision%29))
  (Pawn|Input|AddMovementInput (Transformation|GetActorForwardVector) (Variables|Default|GetScale%20Value) false))

(event EventPlayerMovedRight
  (bind _returnvalue (Transformation|GetActorLocation))
  (bind _returnvalue_2 (Transformation|GetActorLocation))
  (Variables|Default|SetRight_Before (.y _returnvalue_2))
  (Variables|Default|SetRight_After (+ (.y _returnvalue_2) 2e+02))
  (bind _alpha (Timeline|Timeline_0 PlayFromStart)
    (:Update
      (Transformation|SetActorLocation (Math|Vector|MakeVector (.x _returnvalue) (Math|Float|Lerp (Variables|Default|GetRight_Before) (Variables|Default|GetRight_After) _alpha) (.z _returnvalue)) false false))))

(event EventPlayerMovedLeft
  (bind _returnvalue (Transformation|GetActorLocation))
  (bind _returnvalue_2 (Transformation|GetActorLocation))
  (Variables|Default|SetLeft_Before (.y _returnvalue))
  (Variables|Default|SetLeft_After (- (.y _returnvalue) 2e+02))
  (bind _alpha (Timeline|Timeline_1 PlayFromStart)
    (:Update
      (Transformation|SetActorLocation (Math|Vector|MakeVector (.x _returnvalue_2) (Math|Float|Lerp (Variables|Default|GetLeft_Before) (Variables|Default|GetLeft_After) _alpha) (.z _returnvalue_2)) false false))))

(fn ConstructionScript)

(fn IncreaseSpeed
  (bind _charactermovement (Variables|Character|GetCharacterMovement))
  (bind _output_get (Variables|/Script/Engine.CharacterMovementComponent|SetMaxWalkSpeed _charactermovement (+ (* (Variables|/Script/Engine.CharacterMovementComponent|GetMaxWalkSpeed _charactermovement) 0.2) (Variables|/Script/Engine.CharacterMovementComponent|GetMaxWalkSpeed _charactermovement))))
  (Character|LaunchCharacter "30.000000, 0, 0" false false)
  (if (> _output_get (Variables|Default|GetMax%20Speed))
    (Variables|/Script/Engine.CharacterMovementComponent|SetMaxWalkSpeed _charactermovement (Variables|Default|GetMax%20Speed))))