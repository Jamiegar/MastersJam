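; Player character for a lane-based endless runner that auto-runs forward, scoring by distance from the start and counting coins on a HUD widget.
; A/D timelines slide it between lanes, Space jumps and S slams it down mid-air, with doubled gravity while falling.
; Lane moves and jumps are relayed to a Chaser.
; It also handles capped speed increases, an Escape pause menu, and death that locks movement and starts a timer.
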(event Custom|DesplayResults
  (Input|SetInputModeUIOnly (Game|GetPlayerController 0) 0 "DoNotLock")
  (Default|CallPlayerKilled (Variables|Default|GetScore) (Variables|Default|GetCredits)))

(event EventBeginPlay
  (Variables|Default|SetstartPos (Transformation|GetActorLocation))
  (bind _returnvalue (UserInterface|CreateWidget "/Game/UI/coinsandscore/scoreandcoins_widget.scoreandcoins_widget_C"))
  (bind _output_get (Variables|Default|SetGameUI _returnvalue))
  (UserInterface|Viewport|AddtoViewport _output_get 0)
  (Input|SetInputModeGameOnly (Game|GetPlayerController 0)))

(event EventTick
  (params (DeltaSeconds :type Float%20%28single-precision%29))
  (Utilities|FlowControl|Sequence
    (:then_0
      (Development|PrintString (Utilities|String|ToString(Vector) (Transformation|GetActorLocation)) true true "(R=0.000000,G=0.660000,B=1.000000,A=1.000000)" 0.0)
      (if (< (.z (Transformation|GetVelocity)) 0.0)
        (Variables|/Script/Engine.CharacterMovementComponent|SetGravityScale (Variables|Character|GetCharacterMovement) 2.0)
        (else
          (Variables|/Script/Engine.CharacterMovementComponent|SetGravityScale (Variables|Character|GetCharacterMovement) 1.0))))
    (:then_1
      (Pawn|Input|AddMovementInput (Transformation|GetActorForwardVector) (Variables|Movement|GetMoveSpeed) false)
      (CallFunction|AddScore))))

(event Input|KeyboardEvents|A
  (params (Key :type Key%20Structure :default "None"))
  (bind _returnvalue (Transformation|GetActorLocation))
  (bind _returnvalue_2 (Transformation|GetActorLocation))
  (:Pressed
    (if (not (or (Variables|Movement|Getismovingleft?) (Variables|Movement|Getismovingright?)))
      (if (not (<= (.y (Transformation|GetActorLocation)) -2e+02))
        (Variables|Movement|SetLeft%20Before%20Y%20Position (.y _returnvalue_2))
        (Variables|Movement|SetLeft%20After%20Y%20Position (- (.y _returnvalue_2) 2e+02))
        (Variables|Movement|Setismovingleft? true)
        (bind _alpha (Timeline|Timeline_1 PlayFromStart)
          (:Update
            (Transformation|SetActorLocation (Math|Vector|MakeVector (.x _returnvalue) (Math|Float|Lerp (Variables|Movement|GetLeft%20Before%20Y%20Position) (Variables|Movement|GetLeft%20After%20Y%20Position) _alpha) (.z _returnvalue)) false false))
          (:Finished
            (Variables|Movement|Setismovingleft? false)
            (Class|PlayerMovedInterface|PlayerMovedLeft(Message) (Variables|Default|Getchaser))))))))

(event Input|KeyboardEvents|D
  (params (Key :type Key%20Structure :default "None"))
  (bind _returnvalue (Transformation|GetActorLocation))
  (bind _returnvalue_2 (Transformation|GetActorLocation))
  (:Pressed
    (if (not (or (Variables|Movement|Getismovingleft?) (Variables|Movement|Getismovingright?)))
      (if (not (>= (.y (Transformation|GetActorLocation)) 2e+02))
        (Variables|Movement|SetRight%20Before%20Y%20Position (.y _returnvalue))
        (Variables|Movement|SetRight%20After%20Y%20Position (+ (.y _returnvalue) 2e+02))
        (Variables|Movement|Setismovingright? true)
        (bind _alpha (Timeline|Timeline_0 PlayFromStart)
          (:Update
            (Transformation|SetActorLocation (Math|Vector|MakeVector (.x _returnvalue_2) (Math|Float|Lerp (Variables|Movement|GetRight%20Before%20Y%20Position) (Variables|Movement|GetRight%20After%20Y%20Position) _alpha) (.z _returnvalue_2)) false false))
          (:Finished
            (Variables|Movement|Setismovingright? false)
            (Class|PlayerMovedInterface|PlayerMovedRight(Message) (Variables|Default|Getchaser))))))))

(event Input|KeyboardEvents|SpaceBar
  (params (Key :type Key%20Structure :default "None"))
  (:Pressed
    (if (not (Variables|Default|GetisDead))
      (Character|Jump)
      (Class|PlayerJumpedInterface|PlayerJumped(Message) (Variables|Default|Getchaser))))
  (:Released
    (Character|StopJumping)))

(event Input|KeyboardEvents|S
  (params (Key :type Key%20Structure :default "None"))
  (:Pressed
    (if (not (AI|Components|NavMovement|IsMovingonGround (Variables|Character|GetCharacterMovement)))
      (Character|LaunchCharacter (- (Transformation|GetVelocity) "0,0,900.000000") true true))))

(event Input|KeyboardEvents|Escape
  (params (Key :type Key%20Structure :default "None"))
  (:Pressed
    (if (Game|IsGamePaused)
      (CallFunction|ResumeGame)
      (else
        (bind _returnvalue (UserInterface|CreateWidget "/Game/UI/PAUSEMENU/PAUSEMENU_WIDGET.PAUSEMENU_WIDGET_C"))
        (bind _output_get (Variables|Default|SetPauseMenu _returnvalue))
        (UserInterface|Viewport|AddtoViewport _output_get 0)
        (Game|SetGamePaused true)
        (Variables|/Script/Engine.PlayerController|SetbShowMouseCursor (Game|GetPlayerController 0) true)
        (EventDispatchers|BindEventtoResumeButtonClick (Variables|Default|GetPauseMenu) (EventDispatchers|CreateEvent :!event ResumeGame))
        (Input|SetInputModeGameandUI (Game|GetPlayerController 0) (Variables|Default|GetPauseMenu) "DoNotLock" true)))))

(fn ConstructionScript)

(fn IncreaseSpeed
  (bind _charactermovement (Variables|Character|GetCharacterMovement))
  (bind _output_get (Variables|/Script/Engine.CharacterMovementComponent|SetMaxWalkSpeed _charactermovement (+ (* (Variables|/Script/Engine.CharacterMovementComponent|GetMaxWalkSpeed _charactermovement) 0.2) (Variables|/Script/Engine.CharacterMovementComponent|GetMaxWalkSpeed _charactermovement))))
  (if (> _output_get (Variables|Movement|GetMaxSpeed))
    (Variables|/Script/Engine.CharacterMovementComponent|SetMaxWalkSpeed _charactermovement (Variables|Movement|GetMaxSpeed))))

(fn KillPlayer
  (Variables|Movement|Setismovingright? true)
  (Variables|Movement|Setismovingleft? true)
  (Variables|/Script/Engine.CharacterMovementComponent|SetMaxWalkSpeed (Variables|Character|GetCharacterMovement) 0.0)
  (Variables|/Script/Engine.PlayerController|SetbShowMouseCursor (Game|GetPlayerController 0) true)
  (Widget|RemovefromParent (Variables|Default|GetGameUI))
  (Variables|Default|SetisDead true)
  (Utilities|Time|SetTimerbyEvent (EventDispatchers|CreateEvent :!event Custom|DesplayResults) 2.5))

(fn AddCoin
  (bind _result (Math|Integer|IncrementInt (Variables|Default|GetCredits))
    (:%20%20
      (Default|UpdateCoins (Variables|Default|GetGameUI) _result))))

(fn AddScore
  (bind _output_get (Variables|Default|SetScore (/ (Math|Float|Truncate (Math|Vector|VectorLength (- (Variables|Default|GetstartPos) (Transformation|GetActorLocation)))) 200)))
  (Default|UpdateScore (Variables|Default|GetGameUI) _output_get))

(fn ResumeGame
  (Widget|RemovefromParent (Variables|Default|GetPauseMenu))
  (Variables|Default|SetPauseMenu 0)
  (Game|SetGamePaused false)
  (Variables|/Script/Engine.PlayerController|SetbShowMouseCursor (Game|GetPlayerController 0) false)
  (Input|SetInputModeGameOnly (Game|GetPlayerController 0)))